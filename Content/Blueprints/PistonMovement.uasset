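; Piston actor that pushes back and forth on its own through physics forces.
; Every tick, a sine of game time, shaped by Frequency and Acceleration, drives a force along the Pusher component's forward vector.
; The force is applied as an acceleration, so the Pusher's mass does not affect it.
; Leftover input-mapping and debug-print nodes are disconnected and never run.
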(event EventBeginPlay)

(event Collision|EventActorBeginOverlap
  (params (OtherActor :type Actor%20Object%20Reference)))

(event EventTick
  (params (DeltaSeconds :type Float%20%28single-precision%29))
  (Physics|AddForce (Variables|Default|GetPusher) (* (Math|Vector|GetForwardVector (Variables|Default|GetPusher)) (* (Math|Trig|Sin(Radians) (* (Utilities|Time|GetTimeSeconds) (Variables|Default|Getfrequency))) (Variables|Default|Getacceleration))) "None" true))

(event Input|ActionEvents|InputActionUp
  (params (Key :type Key%20Structure)))

(event Input|ActionEvents|InputActionDown
  (params (Key :type Key%20Structure)))

(fn ConstructionScript)