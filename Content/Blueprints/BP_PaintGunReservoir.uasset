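; BP_PaintGunReservoir is a grabbable paint reservoir that loads into the VR paint gun.
; On drop or actor overlap, an unattached reservoir offers itself and its Flex particle template to overlapping BP_VRTool_Paintgun actors, disabling physics once one accepts.
; Pickup unloads it from the gun.
; The construction script tints it through a dynamic material using its Color, and BeginPlay attaches the Flex emitter to its root.
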(event EventBeginPlay
  (Effects|SpawnEmitterAttached "/Game/Blueprints/flexSurfaceEmitterMultColorVM.flexSurfaceEmitterMultColorVM" (Variables|Default|GetRoot) "None" "0, 0, 0" "0, 0, 0" "1.000000,1.000000,1.000000" "SnapToTarget" true "AutoRelease"))

(event Collision|EventActorBeginOverlap
  (params (OtherActor :type Actor%20Object%20Reference))
  (if (== (Variables|Default|GetAttached%20To) 0)
    (bind _array_element (Utilities|Array|ForEachLoopwithBreak (Collision|GetOverlappingActors (Variables|Default|GetRoot) "/Game/Blueprints/BP_VRTool_Paintgun.BP_VRTool_Paintgun_C" :!class /Script/Engine.PrimitiveComponent) :!label _label)
      (:LoopBody
        (bind _asbp_vrtool_paintgun (Utilities|Casting|CastToBP_VRTool_Paintgun _array_element))
        (bind _success (Default|Load _asbp_vrtool_paintgun self "/Game/Blueprints/flexSurfaceEmitterMultColorVM.flexSurfaceEmitterMultColorVM"))
        (if _success
          (Variables|Default|SetAttached%20To _asbp_vrtool_paintgun)
          (Physics|SetSimulatePhysics (Variables|Default|GetRoot) false)
          (goto _label Break))))))

(event EventTick
  (params (DeltaSeconds :type Float%20%28single-precision%29)))

(event EventDrop
  (|CallParentFunction)
  (if (== (Variables|Default|GetAttached%20To) 0)
    (bind _array_element (Utilities|Array|ForEachLoopwithBreak (Collision|GetOverlappingActors (Variables|Default|GetRoot) "/Game/Blueprints/BP_VRTool_Paintgun.BP_VRTool_Paintgun_C" :!class /Script/Engine.PrimitiveComponent) :!label _label)
      (:LoopBody
        (bind _asbp_vrtool_paintgun (Utilities|Casting|CastToBP_VRTool_Paintgun _array_element))
        (bind _success (Default|Load _asbp_vrtool_paintgun self "/Game/Blueprints/flexSurfaceEmitterMultColorVM.flexSurfaceEmitterMultColorVM"))
        (if _success
          (Variables|Default|SetAttached%20To _asbp_vrtool_paintgun)
          (Physics|SetSimulatePhysics (Variables|Default|GetRoot) false)
          (goto _label Break))))))

(event EventPickup
  (params (AttachTo :type Scene%20Component%20Object%20Reference))
  (|CallParentFunction AttachTo)
  (if (!= (Variables|Default|GetAttached%20To) 0)
    (Default|Unload (Variables|Default|GetAttached%20To))
    (Variables|Default|SetAttached%20To 0)))

(fn ConstructionScript
  (bind _tool (Variables|Default|GetTool))
  (bind _returnvalue (Rendering|Material|CreateDynamicMaterialInstance _tool 0 "/Game/Geometry/Meshes/Mat_PaintGunReservoir.Mat_PaintGunReservoir" "None" :!class /Script/Engine.PrimitiveComponent))
  (bind _output_get (Variables|Default|SetDynamic%20Material%20Instance _returnvalue))
  (Rendering|Material|SetVectorParameterValue _output_get "Color" (Variables|Default|GetColor) :!class /Script/Engine.MaterialInstanceDynamic)
  (Rendering|Material|SetMaterial _tool 0 _output_get))