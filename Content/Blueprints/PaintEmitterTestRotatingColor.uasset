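; Test Blueprint for a Flex paint emitter that continuously changes its particle color.
; BeginPlay passes a surface emitter multi-color reference to the Flex particle system controller.
; Each Tick treats the controller's color as a vector and rotates it around Z by a delta-time-scaled angle, so red and green swing while blue stays fixed.
; Disconnected leftover nodes hold paint speed, emission angle and debug print experiments that never run.
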(event EventBeginPlay
  (Variables|/Game/Blueprints/flexParticleSystemController.flexParticleSystemController_C|SetflexSurfaceEmitterMultColorVM (Variables|Default|GetflexParticleSystemController) (Variables|Default|GetflexSurfaceEmitterMultColorVM)))

(event Collision|EventActorBeginOverlap
  (params (OtherActor :type Actor%20Object%20Reference)))

(event EventTick
  (params (DeltaSeconds :type Float%20%28single-precision%29))
  (Variables|/Game/Blueprints/flexParticleSystemController.flexParticleSystemController_C|SetColor (Variables|Default|GetflexParticleSystemController) (Math|Conversions|ToLinearColor(Vector) (Math|Vector|RotateVectorAroundAxis (Math|Conversions|ToVector(LinearColor) (Variables|/Game/Blueprints/flexParticleSystemController.flexParticleSystemController_C|GetColor (Variables|Default|GetflexParticleSystemController))) (* DeltaSeconds 5e+02) "0, 0,1.000000"))))

(fn ConstructionScript)