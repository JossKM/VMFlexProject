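; VR paint gun tool that sprays colored Flex particle paint from its muzzle once a paint actor is loaded.
; Load snaps the paint actor to the attach point, passes its color to the FlexParticleSystemController and spawns the emitter on the muzzle.
; Interact input drives paint speed, which scales muzzle recoil force and looping-audio volume; UnInteract stops both flow and sound.
; Unload detaches and releases the emitter, clearing the loaded state.
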(event EventBeginPlay
  (|CallParentFunction))

(event Collision|EventActorBeginOverlap
  (params (OtherActor :type Actor%20Object%20Reference))
  (|CallParentFunction OtherActor) ; This node is disabled and will not be called.\nDrag off pins to build functionality.
)

(event EventInteract
  (params (amount :type Float%20%28single-precision%29))
  (bind _audio (Variables|Default|GetAudio))
  (bind _muzzle (Variables|Default|GetMuzzle))
  (if (Variables|Default|GetLoaded)
    (bind _output_get (Variables|/Game/Blueprints/flexParticleSystemController.flexParticleSystemController_C|SetPaint%20Speed (Variables|Default|GetflexParticleSystemController) (* amount (Math|Float|Lerp (Variables|Default|GetPaintFlowSpeedMin) (Variables|Default|GetPaintFlowSpeedMax) amount))))
    (Class|PrimitiveComponent|AddForceatLocation (Variables|Default|GetTool) (* (Math|Vector|GetForwardVector _muzzle) (* _output_get (Variables|Default|GetRecoilBySpeed))) (Transformation|GetWorldLocation _muzzle) "None")
    (Audio|Components|Audio|SetVolumeMultiplier _audio (/ _output_get (Variables|Default|GetPaintFlowSpeedMax)) :!class /Script/Engine.AudioComponent)
    (if (not (Audio|Components|Audio|IsPlaying _audio))
      (Audio|Components|Audio|Play _audio 0.0))))

(event EventUnInteract
  (Variables|/Game/Blueprints/flexParticleSystemController.flexParticleSystemController_C|SetPaint%20Speed (Variables|Default|GetflexParticleSystemController) 0.0)
  (Audio|Components|Audio|Stop (Variables|Default|GetAudio)))

(fn ConstructionScript
  (|CallParentFunction))

(fn Load
  (params (Paint%20Actor :type BP%20Paint%20Gun%20Reservoir%20Object%20Reference) (Particles :type Particle%20System%20Object%20Reference))
  (if (Variables|Default|GetLoaded)
    (return false)
    (else
      (Transformation|AttachComponentToComponent Paint%20Actor (Variables|Default|GetAttachPoint) "None" "SnapToTarget" "SnapToTarget" "KeepRelative" true)
      (Variables|/Game/Blueprints/flexParticleSystemController.flexParticleSystemController_C|SetColor (Variables|Default|GetflexParticleSystemController) (Variables|/Game/Blueprints/BP_PaintGunReservoir.BP_PaintGunReservoir_C|GetColor Paint%20Actor))
      (Variables|Default|SetLoaded true)
      (bind _returnvalue (Effects|SpawnEmitterAttached Particles (Variables|Default|GetMuzzle) "None" "0, 0, 0" "0, 0, 0" "1.000000,1.000000,1.000000" "SnapToTarget"))
      (bind _output_get (Variables|Default|SetcurrentParticleSystem _returnvalue))
      (Variables|/Game/Blueprints/flexParticleSystemController.flexParticleSystemController_C|SetflexSurfaceEmitterMultColorVM (Variables|Default|GetflexParticleSystemController) _output_get)
      (Variables|/Game/Blueprints/flexParticleSystemController.flexParticleSystemController_C|SetPaint%20Speed (Variables|Default|GetflexParticleSystemController) 0.0)
      (return true))))

(fn Unload
  (params (Paint%20Actor :type BP%20Paint%20Gun%20Reservoir%20Object%20Reference))
  (Utilities|IsValid (Variables|Default|GetcurrentParticleSystem)
    (:Is%20Valid
      (Transformation|AttachComponentToComponent (Variables|Default|GetcurrentParticleSystem) (Variables|/Game/Blueprints/BP_VRTool.BP_VRTool_C|GetRoot Paint%20Actor) "None" "SnapToTarget" "SnapToTarget" "KeepWorld" true)
      (Variables|Default|SetLoaded false)
      (Transformation|DetachFromComponent (Variables|Default|GetcurrentParticleSystem) "KeepRelative" "KeepRelative" "KeepRelative" true)
      (Variables|Default|SetcurrentParticleSystem 0)
      (Development|PrintString "detach"))))