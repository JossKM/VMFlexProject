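; BP_VRTool is a grabbable VR tool actor with empty ActivateTool and DeactivateTool functions, apparently a base for specific tools.
; Pickup turns off physics on Root and attaches it to the supplied component, snapping location and rotation while keeping world scale.
; Drop restores physics and detaches in place, then runs a short delay that leads nowhere.
; Collision object type changes on the Tool component are left unconnected.
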(event EventBeginPlay)

(event Collision|EventActorBeginOverlap
  (params (OtherActor :type Actor%20Object%20Reference)))

(event EventTick
  (params (DeltaSeconds :type Float%20%28single-precision%29)))

(event EventPickup
  (params (AttachTo :type Scene%20Component%20Object%20Reference))
  (bind _root (Variables|Default|GetRoot))
  (Physics|SetSimulatePhysics _root false)
  (Transformation|AttachComponentToComponent _root AttachTo "None" "SnapToTarget" "SnapToTarget" "KeepWorld" false))

(event EventDrop
  (Physics|SetSimulatePhysics (Variables|Default|GetRoot) true)
  (Transformation|DetachFromActor "KeepWorld" "KeepWorld" "KeepWorld")
  (Utilities|FlowControl|Delay 0.5))

(fn ConstructionScript)

(fn ActivateTool)

(fn DeactivateTool)