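; VR paint gun tool, rapid-fire variant, that sprays paint through a Flex particle system while interacted with.
; When loaded, Interact sets paint speed from the flow range with the blend fixed at minimum, pushes the tool with speed-scaled force along the muzzle's forward vector as recoil, and keeps audio playing.
; UnInteract zeroes paint speed and stops the audio.
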(event EventBeginPlay
  (|CallParentFunction) ; This node is disabled and will not be called.\nDrag off pins to build functionality.
)

(event Collision|EventActorBeginOverlap
  (params (OtherActor :type Actor%20Object%20Reference))
  (|CallParentFunction OtherActor) ; This node is disabled and will not be called.\nDrag off pins to build functionality.
)

(event EventTick
  (params (DeltaSeconds :type Float%20%28single-precision%29))
  (|CallParentFunction DeltaSeconds) ; This node is disabled and will not be called.\nDrag off pins to build functionality.
)

(event EventInteract
  (params (amount :type Float%20%28single-precision%29))
  (bind _audio (Variables|Default|GetAudio))
  (bind _muzzle (Variables|Default|GetMuzzle))
  (if (Variables|Default|GetLoaded)
    (bind _output_get (Variables|/Game/Blueprints/flexParticleSystemController.flexParticleSystemController_C|SetPaint%20Speed (Variables|Default|GetflexParticleSystemController) (* 0.0 (Math|Float|Lerp (Variables|Default|GetPaintFlowSpeedMin) (Variables|Default|GetPaintFlowSpeedMax) 0.0))))
    (Class|PrimitiveComponent|AddForceatLocation (Variables|Default|GetTool) (* (Math|Vector|GetForwardVector _muzzle) (* _output_get (Variables|Default|GetRecoilBySpeed))) (Transformation|GetWorldLocation _muzzle) "None")
    (Audio|Components|Audio|SetVolumeMultiplier _audio 0.0 :!class /Script/Engine.AudioComponent)
    (if (not (Audio|Components|Audio|IsPlaying _audio))
      (Audio|Components|Audio|Play _audio 0.0))))

(event EventUnInteract
  (Variables|/Game/Blueprints/flexParticleSystemController.flexParticleSystemController_C|SetPaint%20Speed (Variables|Default|GetflexParticleSystemController) 0.0)
  (Audio|Components|Audio|Stop (Variables|Default|GetAudio)))

(fn ConstructionScript
  (|CallParentFunction))