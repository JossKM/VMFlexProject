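; BendyTool is a grabbable tool actor that can be picked up and dropped.
; Pickup turns off physics on the Handle, attaches the root component to the supplied component keeping world transform, and prints a debug message.
; It also applies a zero force to the Handle, which has no effect.
; Drop re-enables Handle physics and detaches the actor, and no bending behavior appears in these graphs.
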(event EventBeginPlay)

(event Collision|EventActorBeginOverlap
  (params (OtherActor :type Actor%20Object%20Reference)))

(event EventTick
  (params (DeltaSeconds :type Float%20%28single-precision%29)))

(event EventPickup
  (params (AttachTo :type Scene%20Component%20Object%20Reference))
  (Physics|SetSimulatePhysics (Variables|Default|GetHandle) false)
  (Transformation|AttachComponentToComponent (VehicleSound|GetRootComponent) AttachTo "None" "KeepWorld" "KeepWorld" "KeepWorld" false)
  (Class|PrimitiveComponent|AddForceatLocation (Variables|Default|GetHandle) "0, 0, 0" "0, 0, 0" "None")
  (Development|PrintString "you grabbed me!"))

(event EventDrop
  (Physics|SetSimulatePhysics (Variables|Default|GetHandle) true)
  (Transformation|DetachFromActor "KeepWorld" "KeepWorld" "KeepWorld"))

(fn ConstructionScript)